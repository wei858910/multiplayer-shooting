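; BP_Bruch is a brush scene component that feeds draw data to BP_DrawBoard, apparently for snow deformation.
; On BeginPlay it finds and caches the draw board actor.
; Each Tick, it line-traces down from its world location over the snow height on the Visibility channel.
; On a hit, it passes its position, brush size and offset-adjusted hit distance as height to the board's AddDraw.
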(event EventBeginPlay
  (bind _returnvalue (Actor|GetActorOfClass "/Game/Test/Snow/BP_DrawBoard.BP_DrawBoard_C"))
  (Variables|Default|SetDrawBoard _returnvalue))

(event EventTick
  (params (DeltaSeconds :type Float%20%28single-precision%29))
  (bind _returnvalue (Transformation|GetWorldLocation))
  (bind _drawboard (Variables|Default|GetDrawBoard))
  (Utilities|IsValid _drawboard
    (:Is%20Valid
      (bind (_outhit _returnvalue_2) (Collision|LineTraceByChannel _returnvalue (- _returnvalue (Math|Vector|MakeVector 0.0 0.0 (Variables|Default|GetSnow%20Heigh))) "TraceTypeQuery1" false 0 "None"))
      (if _returnvalue_2
        (Default|AddDraw _drawboard (Utilities|Struct|MakeS_BruchInfo _returnvalue (Variables|Default|GetSize) (- (.Distance (Collision|BreakHitResult _outhit)) (Variables|Default|GetTrace%20Offset))))))))