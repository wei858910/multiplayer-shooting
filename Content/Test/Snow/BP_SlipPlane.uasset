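; BP_SlipPlane is a snow test actor that estimates the cross-sectional area where its Plane cuts a referenced static mesh actor.
; Its construction script copies the mesh into a temporary procedural mesh, slices it with a new cap section, and reads section 1.
; It sums cross-product triangle areas into CrossSectionalArea, prints it, and destroys the temporary component.
; The loop steps one index at a time, not three, so triangles are misread.
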(event EventBeginPlay)

(fn ConstructionScript
  (bind _staticmesh (Variables|Default|GetStaticMesh))
  (bind _plane (Variables|Default|GetPlane))
  (bind _returnvalue (AddComponent|AddProceduralMeshComponent true (Transformation|GetActorTransform _staticmesh)))
  (Class|KismetProceduralMeshLibrary|CopyProceduralMeshfromStaticMeshComponent (Variables|/Script/Engine.StaticMeshActor|GetStaticMeshComponent _staticmesh) 0 _returnvalue false)
  (Class|KismetProceduralMeshLibrary|SliceProceduralMesh _returnvalue (Transformation|GetWorldLocation _plane) (Math|Vector|GetUpVector _plane) false "CreateNewSectionForCap")
  (bind (_vertices _triangles) (Class|KismetProceduralMeshLibrary|GetSectionfromProceduralMesh _returnvalue 1))
  (Variables|Default|SetCross%20Sectional%20Area 0.0)
  (for _index (range 0 (- (/ (Utilities|Array|Length _triangles) 3) 1))
    (Variables|Default|SetCross%20Sectional%20Area (+ (Variables|Default|GetCross%20Sectional%20Area) (/ (Math|Vector|VectorLength (Math|Vector|CrossProduct (- (Utilities|Array|Get(acopy) _vertices (Utilities|Array|Get(acopy) _triangles (+ _index 0))) (Utilities|Array|Get(acopy) _vertices (Utilities|Array|Get(acopy) _triangles (+ _index 1)))) (- (Utilities|Array|Get(acopy) _vertices (Utilities|Array|Get(acopy) _triangles (+ _index 0))) (Utilities|Array|Get(acopy) _vertices (Utilities|Array|Get(acopy) _triangles (+ _index 2)))))) 2.0))))
  (Components|DestroyComponent _returnvalue)
  (Development|PrintString (Utilities|String|ToString(Float) (Variables|Default|GetCross%20Sectional%20Area))))