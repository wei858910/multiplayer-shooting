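; Snow deformation board that records height brush stamps into a render target covering a square of world around the player.
; Each tick it snaps the canvas to the player in whole-texel steps and updates MPC_Snow and its plane.
; It redraws RT_Snow through a UV-offset translation material, stamps brushes queued by AddDraw, then copies the result to RT_SnowSave.
; This double buffer with texel snapping forms a scrolling window that follows the player.
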(event Custom|AddDraw
  (params (BruchInfo :type S%20Bruch%20Info%20Structure))
  (Utilities|Array|Add (Variables|Default|GetBruch%20Info) BruchInfo))

(event EventBeginPlay
  (bind _canvas_size (Variables|Default|GetCanvas%20Size))
  (bind _canvas_position (Variables|Default|GetCanvas%20Position))
  (Rendering|ClearRenderTarget2D "/Game/Test/Snow/RT_Snow.RT_Snow")
  (Rendering|ClearRenderTarget2D "/Game/Test/Snow/RT_SnowSave.RT_SnowSave")
  (Rendering|Material|SetVectorParameterValue "/Game/Test/Snow/MPC_Snow.MPC_Snow" "PositionSize" (Utilities|Struct|MakeLinearColor (.x _canvas_position) (.y _canvas_position) (.x _canvas_size) (.y _canvas_size)) :!class /Script/Engine.KismetMaterialLibrary)
  (Variables|Default|SetCanvasPixelSize (/ (Variables|Default|GetCanvas%20Size) (Variables|Default|GetRTSize))))

(event EventTick
  (params (DeltaSeconds :type Float%20%28single-precision%29))
  (Rendering|ClearRenderTarget2D "/Game/Test/Snow/RT_Snow.RT_Snow")
  (CallFunction|ChangePosition (Math|Conversions|ToVector2D(Vector) (Transformation|GetActorLocation (Game|Player|GetPlayerPawn 0))))
  (CallFunction|TranslationSnow)
  (CallFunction|DrawSnow)
  (CallFunction|CopySnow))

(fn ConstructionScript
  (Transformation|SetWorldTransform (Variables|Default|GetPlane) (Math|Transform|MakeTransform (Math|Conversions|ToVector(Vector2D) (Variables|Default|GetCanvas%20Position)) "0, 0, 0" (Math|Conversions|ToVector(Vector2D) (/ (Variables|Default|GetCanvas%20Size) "(X=100.000000,Y=100.000000)") 1.0)) false false))

(fn WorldPositiontoUVTest
  (params (Position :type Vector))
  (bind (_x _y) (Class|KismetMathLibrary|BreakVector3f Position))
  (return (+ (/ (- (Math|Vector2D|MakeVector2D _x _y) (Variables|Default|GetCanvas%20Position)) (Variables|Default|GetCanvas%20Size)) "(X=0.500000,Y=0.500000)")))

(fn WorldPositiontoUV
  (params (Burch%20Position :type Vector) (Bruch%20Size :type Vector%202D%20Structure))
  (bind (_x _y) (Class|KismetMathLibrary|BreakVector3f Burch%20Position))
  (bind _canvaspixelsize (Variables|Default|GetCanvasPixelSize))
  (bind _returnvalue (/ Bruch%20Size _canvaspixelsize))
  (return (- (/ (+ (- (Math|Vector2D|MakeVector2D _x _y) (Variables|Default|GetCanvas%20Position)) (/ (Variables|Default|GetCanvas%20Size) "(X=2.000000,Y=2.000000)")) (Variables|Default|GetCanvasPixelSize)) (/ _returnvalue "(X=2.000000,Y=2.000000)")) _returnvalue))

(fn ChangePosition
  (params (Position :type Vector%202D%20Structure))
  (bind _canvaspixelsize (Variables|Default|GetCanvasPixelSize))
  (bind _canvas_size (Variables|Default|GetCanvas%20Size))
  (bind _returnvalue (/ Position _canvaspixelsize))
  (bind (_x _y) (Math|Vector2D|BreakVector2D _returnvalue))
  (Variables|Default|SetCanvas%20LastPosition (Variables|Default|GetCanvas%20Position))
  (Variables|Default|SetCanvas%20Position (* (Math|Vector2D|MakeVector2D (Math|Conversions|ToFloat(Integer) (Math|Float|Floor _x)) (Math|Conversions|ToFloat(Integer) (Math|Float|Floor _y))) (Variables|Default|GetCanvasPixelSize)))
  (Rendering|Material|SetVectorParameterValue "/Game/Test/Snow/MPC_Snow.MPC_Snow" "PositionSize" (Utilities|Struct|MakeLinearColor (.x (Variables|Default|GetCanvas%20Position)) (.y (Variables|Default|GetCanvas%20Position)) (.x _canvas_size) (.y _canvas_size)) :!class /Script/Engine.KismetMaterialLibrary)
  (Transformation|SetWorldTransform (Variables|Default|GetPlane) (Math|Transform|MakeTransform (Math|Conversions|ToVector(Vector2D) (Variables|Default|GetCanvas%20Position)) "0, 0, 0" (Math|Conversions|ToVector(Vector2D) (/ (Variables|Default|GetCanvas%20Size) "(X=100.000000,Y=100.000000)") 1.0)) false false))

(fn CopySnow
  (bind (_canvas _size _context) (Rendering|BeginDrawCanvastoRenderTarget "/Game/Test/Snow/RT_SnowSave.RT_SnowSave"))
  (Canvas|DrawTexture :self _canvas :RenderTexture "/Game/Test/Snow/RT_Snow.RT_Snow" :ScreenSize _size :CoordinateSize "(X=1.000000,Y=1.000000)" :RenderColor "(R=1.000000,G=1.000000,B=1.000000,A=0.000000)" :BlendMode "BLEND_Opaque" :PivotPoint "(X=0.500000,Y=0.500000)")
  (Rendering|EndDrawCanvastoRenderTarget _context))

(fn DrawSnow
  (bind _snow_heigh (Variables|Default|GetSnow%20Heigh))
  (bind _canvas_position (Variables|Default|GetCanvas%20Position))
  (bind _canvas_lastposition (Variables|Default|GetCanvas%20LastPosition))
  (bind _canvas_size (Variables|Default|GetCanvas%20Size))
  (bind _returnvalue (- _canvas_position _canvas_lastposition))
  (bind _returnvalue_2 (/ _returnvalue _canvas_size))
  (bind (_x _y) (Math|Vector2D|BreakVector2D _returnvalue_2))
  (bind _returnvalue_3 (Rendering|Material|CreateDynamicMaterialInstance "/Game/Test/Snow/M_DrawSnow.M_DrawSnow" "None" "None" :!class /Script/Engine.KismetMaterialLibrary))
  (Rendering|Material|SetVectorParameterValue _returnvalue_3 "UVOffset" (Utilities|Struct|MakeLinearColor _x _y 0.0 0.0) :!class /Script/Engine.MaterialInstanceDynamic)
  (bind (_canvas _size _context) (Rendering|BeginDrawCanvastoRenderTarget "/Game/Test/Snow/RT_Snow.RT_Snow"))
  (for _array_element (Variables|Default|GetBruch%20Info)
    (Rendering|Material|SetScalarParameterValue _returnvalue_3 "SnowHeigh" (- 1.0 (/ (- _snow_heigh (.Heigh (Utilities|Struct|BreakS_BruchInfo _array_element))) _snow_heigh)) :!class /Script/Engine.MaterialInstanceDynamic)
    (Canvas|DrawMaterial :self _canvas :RenderMaterial _returnvalue_3 :ScreenPosition (.ScreenPosition (CallFunction|WorldPositiontoUV (.BruchPosition (Utilities|Struct|BreakS_BruchInfo _array_element)) (.BruchSize (Utilities|Struct|BreakS_BruchInfo _array_element)))) :ScreenSize (.ScreenSize (CallFunction|WorldPositiontoUV (.BruchPosition (Utilities|Struct|BreakS_BruchInfo _array_element)) (.BruchSize (Utilities|Struct|BreakS_BruchInfo _array_element)))) :CoordinateSize "(X=1.000000,Y=1.000000)" :PivotPoint "(X=0.500000,Y=0.500000)"))
  (Rendering|EndDrawCanvastoRenderTarget _context)
  (Utilities|Array|Clear (Variables|Default|GetBruch%20Info)))

(fn TranslationSnow
  (bind _canvas_size (Variables|Default|GetCanvas%20Size))
  (bind _canvas_position (Variables|Default|GetCanvas%20Position))
  (bind _canvas_lastposition (Variables|Default|GetCanvas%20LastPosition))
  (bind _returnvalue (- _canvas_position _canvas_lastposition))
  (bind _returnvalue_2 (/ _returnvalue _canvas_size))
  (bind (_x _y) (Math|Vector2D|BreakVector2D _returnvalue_2))
  (bind _returnvalue_3 (Rendering|Material|CreateDynamicMaterialInstance "/Game/Test/Snow/M_Translation.M_Translation" "None" "None" :!class /Script/Engine.KismetMaterialLibrary))
  (Rendering|Material|SetVectorParameterValue _returnvalue_3 "UVOffset" (Utilities|Struct|MakeLinearColor _x _y 0.0 0.0) :!class /Script/Engine.MaterialInstanceDynamic)
  (Rendering|DrawMaterialtoRenderTarget "/Game/Test/Snow/RT_Snow.RT_Snow" _returnvalue_3))