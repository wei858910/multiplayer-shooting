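; Lobby GameMode that keeps a list of the connected player controllers.
; PostLogin adds each controller uniquely, and OnLogout removes it, then calls UpdatePlayerUI on that exiting controller if it is a BP_Lobby_Controller.
; FindPlayerControllerByID searches the list for the controller whose possessed BP_BlasterCharacter has the matching PlayerID, stopping early if a pawn fails that cast.
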(event EventPostLogin
  (params (NewPlayer :type Player%20Controller%20Object%20Reference))
  (Utilities|Array|AddUnique (Variables|Default|GetPlayerControllers) NewPlayer))

(event EventOnLogout
  (params (ExitingController :type Controller%20Object%20Reference))
  (bind _asplayer_controller (Utilities|Casting|CastToPlayerController ExitingController))
  (Utilities|Array|RemoveItem (Variables|Default|GetPlayerControllers) _asplayer_controller)
  (bind _asbp_lobby_controller (Utilities|Casting|CastToBP_Lobby_Controller _asplayer_controller))
  (Default|UpdatePlayerUI _asbp_lobby_controller))

(fn ConstructionScript)

(fn FindPlayerControllerbyID
  (params (PlayerID :type String))
  (for _array_element (Variables|Default|GetPlayerControllers)
    (bind _asbp_blaster_character (Utilities|Casting|CastToBP_BlasterCharacter (Pawn|GetControlledPawn _array_element)))
    (if (Utilities|Enum|Equal(Enum) (Variables|/Game/Blueprints/Character/BP_BlasterCharacter.BP_BlasterCharacter_C|GetPlayerID _asbp_blaster_character) PlayerID)
      (return _array_element)))
  (return 0))