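; Player controller for the multiplayer lobby that creates the lobby UI and handles the player list, chat and session exit.
; On BeginPlay it sends the GameInstance player name to the server, which spawns and possesses a Blaster character with a timestamp-based ID.
; The server gathers names and IDs from the GameMode's controllers and relays them, like chat messages, to each client's widget.
; Client events also show a loading screen or destroy the session and open the main menu.
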(event Custom|Server_SpawnCharacter
  (params (PlayerName :type Text))
  (bind _returnvalue (Math|DateTime|Now))
  (bind _returnvalue_2 (Utilities|String|ToString(Integer) (.day _returnvalue)))
  (bind _returnvalue_3 (Utilities|String|ToString(Integer) (.hour _returnvalue)))
  (bind _returnvalue_4 (Utilities|String|ToString(Integer) (.minute _returnvalue)))
  (bind _returnvalue_5 (Utilities|String|ToString(Integer) (.second _returnvalue)))
  (bind _returnvalue_6 (Utilities|String|ToString(Integer) (.millisecond _returnvalue)))
  (bind _returnvalue_7 (Utilities|String|ToString(Integer) (.year _returnvalue)))
  (bind _returnvalue_8 (Utilities|String|ToString(Integer) (.month _returnvalue)))
  (bind _returnvalue_9 (Utilities|String|Append _returnvalue_7 _returnvalue_8 _returnvalue_2 _returnvalue_3 _returnvalue_4 _returnvalue_5 _returnvalue_6))
  (bind _returnvalue_10 (Actor|GetActorOfClass "/Script/Engine.PlayerStart"))
  (Utilities|IsValid _returnvalue_10
    (:Is%20Valid
      (bind _returnvalue_11 (Game|SpawnActorfromClass "/Game/Blueprints/Character/BP_BlasterCharacter.BP_BlasterCharacter_C" (Transformation|GetActorTransform _returnvalue_10) "Undefined" "MultiplyWithRoot" 0 PlayerName _returnvalue_9 0))
      (Pawn|Possess _returnvalue_11)
      (CallFunction|UpdatePlayerUI))
    (:Is%20Not%20Valid
      (bind _returnvalue_12 (Game|SpawnActorfromClass "/Game/Blueprints/Character/BP_BlasterCharacter.BP_BlasterCharacter_C" (Math|Transform|MakeTransform "0, 0, 0" "0, 0, 0" "1.000000,1.000000,1.000000") "Undefined" "MultiplyWithRoot" 0 PlayerName _returnvalue_9 0))
      (Pawn|Possess _returnvalue_12)
      (CallFunction|UpdatePlayerUI))))

(event Custom|Client_UpdatePlayerUI
  (params (PlayerNames :type Array%20of%20Texts) (PlayerIDs :type Array%20of%20Strings))
  (Utilities|FlowControl|Delay 0.2)
  (Default|UpdatePlayerList (Variables|Default|GetLobby_UI) PlayerNames PlayerIDs))

(event Custom|Client_QuitSession
  (|DestroyRoomSession
    (:OnSuccess
      (Game|OpenLevel(byName) "/Game/Menu/Maps/MainMenuMap"))))

(event Custom|Client_GameLoading
  (bind _returnvalue (CallFunction|FUNLFastCreateWidget "/Maple_FastSetting/UMG/Loading/UMG_Loading_OnlyText.UMG_Loading_OnlyText_C" 10))
  (UserInterface|Viewport|AddtoViewport _returnvalue 0))

(event Custom|Server_SendMessage
  (params (Message :type Text))
  (bind _asbp_lobby_game_mode (Utilities|Casting|CastToBP_Lobby_GameMode (Game|GetGameMode)))
  (for _array_element (Variables|/Game/Menu/Lobby/BP_Lobby_GameMode.BP_Lobby_GameMode_C|GetPlayerControllers _asbp_lobby_game_mode)
    (bind _asbp_lobby_controller (Utilities|Casting|CastToBP_Lobby_Controller _array_element))
    (CallFunction|ClientSendMessage _asbp_lobby_controller Message)))

(event Custom|Client_SendMessage
  (params (Message :type Text))
  (Default|AppendMssage (Variables|Default|GetLobby_UI) Message))

(event EventBeginPlay
  (if (Pawn|IsLocalPlayerController)
    (bind _returnvalue (UserInterface|CreateWidget "/Game/Menu/UI/WBP_Lobby.WBP_Lobby_C" self))
    (UserInterface|Viewport|AddtoViewport _returnvalue 0)
    (Variables|Default|SetLobby_UI _returnvalue)
    (Variables|Default|SetbShowMouseCursor true)
    (bind _asbp_lobby_game_instance (Utilities|Casting|CastToBP_Lobby_GameInstance (Game|GetGameInstance)))
    (CallFunction|ServerSpawnCharacter (Variables|/Game/Menu/BP_Lobby_GameInstance.BP_Lobby_GameInstance_C|GetPlayerName _asbp_lobby_game_instance))))

(fn ConstructionScript)

(fn UpdatePlayerUI
  (bind _returnvalue (Game|GetGameMode))
  (bind _asbp_lobby_game_mode (Utilities|Casting|CastToBP_Lobby_GameMode _returnvalue))
  (bind _playercontrollers (Variables|/Game/Menu/Lobby/BP_Lobby_GameMode.BP_Lobby_GameMode_C|GetPlayerControllers _asbp_lobby_game_mode))
  (if (Ability|HasAuthority)
    (for _array_element _playercontrollers
      (bind _asbp_blaster_character (Utilities|Casting|CastToBP_BlasterCharacter (Pawn|GetControlledPawn _array_element)))
      (Utilities|Array|Add (LocalVariables|GetPlayerNames) (Variables|/Game/Blueprints/Character/BP_BlasterCharacter.BP_BlasterCharacter_C|GetPlayerName _asbp_blaster_character))
      (Utilities|Array|Add (LocalVariables|GetPlayerIDs) (Variables|/Game/Blueprints/Character/BP_BlasterCharacter.BP_BlasterCharacter_C|GetPlayerID _asbp_blaster_character)))
    (for _array_element_2 _playercontrollers
      (bind _asbp_lobby_controller (Utilities|Casting|CastToBP_Lobby_Controller _array_element_2))
      (CallFunction|ClientUpdatePlayerUI _asbp_lobby_controller (LocalVariables|GetPlayerNames) (LocalVariables|GetPlayerIDs)))))